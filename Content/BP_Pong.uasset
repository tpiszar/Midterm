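; BP_Pong runs the match flow for a two-player Pong game, from start to victory.
; On BeginPlay it shows the score widget and spawns BP_Ball at a start transform after a short delay.
; AddScore updates the tally and widget, calling Victory when either player reaches 11.
; Victory shows the end widget, switched to blue winner for player two, ends the score widget and pauses the game.
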(event EventBeginPlay
  (bind _returnvalue (UserInterface|CreateWidget "/Game/ScoreWidget.ScoreWidget_C"))
  (bind _output_get (Variables|Default|SetScoreWidget _returnvalue))
  (UserInterface|Viewport|AddtoViewport _output_get 0)
  (Utilities|FlowControl|Delay 3.0)
  (Game|SpawnActorfromClass "/Game/BP_Ball.BP_Ball_C" (Variables|Default|GetStartTransform) "Undefined" "MultiplyWithRoot" 0 0))

(event EventTick
  (params (DeltaSeconds :type Float%20%28single-precision%29)))

(fn ConstructionScript)

(fn AddScore
  (params (Player1 :type Boolean))
  (if Player1
    (bind _output_get (Variables|Default|SetP1_Score (+ (Variables|Default|GetP1_Score) 1)))
    (else
      (bind _output_get_2 (Variables|Default|SetP2_Score (+ (Variables|Default|GetP2_Score) 1)))))
  (bind _asscore_widget (Utilities|Casting|CastToScoreWidget (Variables|Default|GetScoreWidget)))
  (Default|UpdateScore _asscore_widget _output_get _output_get_2)
  (if (== (Variables|Default|GetP1_Score) 11)
    (CallFunction|Victory true)
    (elif (== (Variables|Default|GetP2_Score) 11)
      (CallFunction|Victory false))))

(fn Victory
  (params (Player1 :type Boolean))
  (bind _returnvalue (UserInterface|CreateWidget "/Game/EndWidget.EndWidget_C"))
  (if Player1
    _
    (else
      (Default|BlueWinner _returnvalue)))
  (UserInterface|Viewport|AddtoViewport _returnvalue 0)
  (bind _asscore_widget (Utilities|Casting|CastToScoreWidget (Variables|Default|GetScoreWidget)))
  (Default|End _asscore_widget)
  (Game|SetGamePaused true))