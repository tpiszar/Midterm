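; BP_BlueGoal is a Pong goal that scores when an actor tagged Ball overlaps its static mesh.
; It disables the ball's collision and passes its Player1 flag to AddScore on the BP_Pong game mode.
; After a delay, it destroys the ball and spawns a new BP_Ball at StartTransform.
; The OtherPlayer function sets Player1 to false, though nothing in this Blueprint calls it.
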(event OnComponentBeginOverlap(StaticMeshComponent)
  (params (OverlappedComponent :type Primitive%20Component%20Object%20Reference) (OtherActor :type Actor%20Object%20Reference) (OtherComp :type Primitive%20Component%20Object%20Reference) (OtherBodyIndex :type Integer) (bFromSweep :type Boolean) (SweepResult :type Hit%20Result%20Structure%20%28by%20ref%29))
  (if (Actor|ActorHasTag OtherActor "Ball")
    (Collision|SetActorEnableCollision OtherActor false)
    (bind _asbp_pong (Utilities|Casting|CastToBP_Pong (Game|GetGameMode)))
    (Default|AddScore _asbp_pong (Variables|Default|GetPlayer1))
    (Utilities|FlowControl|Delay (Variables|Default|GetDelay))
    (Actor|DestroyActor OtherActor)
    (Game|SpawnActorfromClass "/Game/BP_Ball.BP_Ball_C" (Variables|Default|GetStartTransform) "Undefined" "MultiplyWithRoot" 0 0)))

(event EventBeginPlay)

(event Collision|EventActorBeginOverlap
  (params (OtherActor :type Actor%20Object%20Reference)))

(event EventTick
  (params (DeltaSeconds :type Float%20%28single-precision%29)))

(fn ConstructionScript)

(fn OtherPlayer
  (Variables|Default|SetPlayer1 false))