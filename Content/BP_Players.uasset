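; BP_Players is a single pawn that drives four paddles for two local players, one horizontal and one vertical paddle each.
; On BeginPlay it is possessed by the first player controller, shows the cursor and assigns the BP_Paddle actors by GetAllActorsOfClass index, so roles depend on that order.
; Axis inputs move each paddle along its right or forward vector, scaled by Speed and delta time and clamped to the arena bounds.
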(event EventBeginPlay
  (bind _returnvalue (Game|GetPlayerController 0))
  (Pawn|Possess _returnvalue self)
  (Variables|/Script/Engine.PlayerController|SetbShowMouseCursor _returnvalue true)
  (bind _outactors (Actor|GetAllActorsOfClass "/Game/BP_Paddle.BP_Paddle_C"))
  (for (_array_element _array_index) _outactors
    (if (== _array_index 0)
      (Variables|Default|SetP1LR _array_element)
      (elif (== _array_index 1)
        (Variables|Default|SetP2LR _array_element)
        (elif (== _array_index 2)
          (Variables|Default|SetP1UD _array_element)
          (elif (== _array_index 3)
            (Variables|Default|SetP2UD _array_element)))))))

(event Collision|EventActorBeginOverlap
  (params (OtherActor :type Actor%20Object%20Reference)))

(event EventTick
  (params (DeltaSeconds :type Float%20%28single-precision%29)))

(event Input|AxisEvents|InputAxisP1_Horizontal
  (params (AxisValue :type Float%20%28single-precision%29))
  (bind _returnvalue (Utilities|Time|GetWorldDeltaSeconds))
  (bind _p1lr (Variables|Default|GetP1LR))
  (bind _speed (Variables|Default|GetSpeed))
  (bind _returnvalue_2 (Transformation|GetActorLocation _p1lr))
  (bind _returnvalue_3 (Transformation|GetActorRightVector _p1lr))
  (bind _returnvalue_4 (* AxisValue _returnvalue _speed))
  (bind _returnvalue_5 (* _returnvalue_3 _returnvalue_4))
  (bind _returnvalue_6 (+ _returnvalue_2 _returnvalue_5))
  (bind (_x _y _z) (Math|Vector|BreakVector _returnvalue_6))
  (Transformation|SetActorLocation _p1lr (Math|Vector|MakeVector _x (Math|Float|Clamp(Float) _y -2.95e+03 2.95e+03) _z) false false))

(event Input|AxisEvents|InputAxisP2_Horizontal
  (params (AxisValue :type Float%20%28single-precision%29))
  (bind _returnvalue (Utilities|Time|GetWorldDeltaSeconds))
  (bind _p2lr (Variables|Default|GetP2LR))
  (bind _speed (Variables|Default|GetSpeed))
  (bind _returnvalue_2 (Transformation|GetActorLocation _p2lr))
  (bind _returnvalue_3 (Transformation|GetActorRightVector _p2lr))
  (bind _returnvalue_4 (* AxisValue _returnvalue _speed))
  (bind _returnvalue_5 (* _returnvalue_3 _returnvalue_4))
  (bind _returnvalue_6 (+ _returnvalue_2 _returnvalue_5))
  (bind (_x _y _z) (Math|Vector|BreakVector _returnvalue_6))
  (Transformation|SetActorLocation _p2lr (Math|Vector|MakeVector _x (Math|Float|Clamp(Float) _y -2.95e+03 2.95e+03) _z) false false))

(event Input|AxisEvents|InputAxisP1_Vertical
  (params (AxisValue :type Float%20%28single-precision%29))
  (bind _returnvalue (Utilities|Time|GetWorldDeltaSeconds))
  (bind _p1ud (Variables|Default|GetP1UD))
  (bind _speed (Variables|Default|GetSpeed))
  (bind _returnvalue_2 (Transformation|GetActorLocation _p1ud))
  (bind _returnvalue_3 (Transformation|GetActorForwardVector _p1ud))
  (bind _returnvalue_4 (* AxisValue _returnvalue _speed))
  (bind _returnvalue_5 (* _returnvalue_3 _returnvalue_4))
  (bind _returnvalue_6 (+ _returnvalue_2 _returnvalue_5))
  (bind (_x _y _z) (Math|Vector|BreakVector _returnvalue_6))
  (Transformation|SetActorLocation _p1ud (Math|Vector|MakeVector (Math|Float|Clamp(Float) _x -2.95e+03 2.95e+03) _y _z) false false))

(event Input|AxisEvents|InputAxisP2_Vertical
  (params (AxisValue :type Float%20%28single-precision%29))
  (bind _returnvalue (Utilities|Time|GetWorldDeltaSeconds))
  (bind _speed (Variables|Default|GetSpeed))
  (bind _p2ud (Variables|Default|GetP2UD))
  (bind _returnvalue_2 (Transformation|GetActorForwardVector _p2ud))
  (bind _returnvalue_3 (Transformation|GetActorLocation _p2ud))
  (bind _returnvalue_4 (* AxisValue _returnvalue _speed))
  (bind _returnvalue_5 (* _returnvalue_2 _returnvalue_4))
  (bind _returnvalue_6 (+ _returnvalue_3 _returnvalue_5))
  (bind (_x _y _z) (Math|Vector|BreakVector _returnvalue_6))
  (Transformation|SetActorLocation _p2ud (Math|Vector|MakeVector (Math|Float|Clamp(Float) _x -2.95e+03 2.95e+03) _y _z) false false))

(fn ConstructionScript)