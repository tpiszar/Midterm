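; BP_Ball is a physics ball that launches itself in a random horizontal direction when play begins.
; BeginPlay builds a normalized X/Y vector from random floats, signed by Switch1 and Switch2, then applies it times Magnitude as a velocity-change impulse on the static mesh.
; Both random coin flips set Switch1 to negative, so Switch2 keeps its default sign.
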(event EventBeginPlay
  (if (Math|Random|RandomBool)
    (Variables|Default|SetSwitch1 -1))
  (if (Math|Random|RandomBool)
    (Variables|Default|SetSwitch1 -1))
  (Physics|AddImpulse (Variables|Debug|GetStaticMeshComponent) (* (Math|Vector|Normalize (Math|Vector|MakeVector (* (Math|Random|RandomFloatinRange 0.25 0.75) (Variables|Default|GetSwitch1)) (* (Math|Random|RandomFloatinRange 0.25 0.75) (Variables|Default|GetSwitch2)) 0.0)) (Variables|Default|GetMagnitude)) "None" true))

(event Collision|EventActorBeginOverlap
  (params (OtherActor :type Actor%20Object%20Reference)))

(event EventTick
  (params (DeltaSeconds :type Float%20%28single-precision%29)))

(fn ConstructionScript)